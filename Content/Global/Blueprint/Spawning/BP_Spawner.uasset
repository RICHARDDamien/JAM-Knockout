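; BP_Spawner populates the level with BP_PNJ characters at BeginPlay, after destroying any already placed.
; It spawns them at random reachable navmesh points within Radius, with random yaw.
; UseGI selects the local Amount when true, otherwise GI_Jam's AmountOfLovers, which is also debug-printed.
; When UseGI is false, a final pass destroys or spawns BP_PNJs until their count matches AmountOfLovers.
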(event EventBeginPlay
  (bind _returnvalue (Game|GetGameInstance))
  (bind _asgi_jam (Utilities|Casting|CastToGI_Jam _returnvalue))
  (bind _amountoflovers (Variables|/Game/Global/Blueprint/GI_Jam.GI_Jam_C|GetAmountOfLovers _asgi_jam))
  (bind _outactors (Actor|GetAllActorsOfClass "/Game/Global/Blueprint/Player/BP_PNJ.BP_PNJ_C"))
  (for _array_element _outactors
    (Actor|DestroyActor _array_element))
  (Development|PrintString (Utilities|String|ToString(Integer) _amountoflovers) true true "(R=1.000000,G=0.000000,B=0.068094,A=1.000000)" 5e+01)
  (Utilities|FlowControl|Delay 0.2)
  (for _index (range 0 (Math|Integer|SelectInt (Variables|Default|GetAmount) _amountoflovers (Variables|Default|GetUseGI)))
    (Game|SpawnActorfromClass "/Game/Global/Blueprint/Player/BP_PNJ.BP_PNJ_C" (Math|Transform|MakeTransform (.RandomLocation (AI|Navigation|GetRandomReachablePointinRadius (Transformation|GetActorLocation) (Variables|Default|GetRadius) 0 0)) (Math|Rotator|MakeRotator 0.0 0.0 (.yaw (Math|Random|RandomRotator true))) "1.000000,1.000000,1.000000") "Undefined" "MultiplyWithRoot" 0 false 0))
  (if (not (Variables|Default|GetUseGI))
    (bind _outactors_2 (Actor|GetAllActorsOfClass "/Game/Global/Blueprint/Player/BP_PNJ.BP_PNJ_C"))
    (if (not (== (Utilities|Array|Length _outactors_2) _amountoflovers))
      (if (> (- (Utilities|Array|Length _outactors_2) _amountoflovers) 0)
        (for _index_2 (range 0 (- (Math|Integer|Absolute(Integer) (- (Utilities|Array|Length _outactors_2) _amountoflovers)) 1))
          (Actor|DestroyActor (Utilities|Array|Get(acopy) _outactors_2 _index_2)))
        (else
          (for _index_3 (range 0 (- (Math|Integer|Absolute(Integer) (- (Utilities|Array|Length _outactors_2) _amountoflovers)) 1))
            (Game|SpawnActorfromClass "/Game/Global/Blueprint/Player/BP_PNJ.BP_PNJ_C" (Math|Transform|MakeTransform (.RandomLocation (AI|Navigation|GetRandomReachablePointinRadius (Transformation|GetActorLocation) (Variables|Default|GetRadius) 0 0)) (Math|Rotator|MakeRotator 0.0 0.0 (.yaw (Math|Random|RandomRotator true))) "1.000000,1.000000,1.000000") "Undefined" "MultiplyWithRoot" 0 false 0)))))))

(event Collision|EventActorBeginOverlap
  (params (OtherActor :type Actor%20Object%20Reference)))

(fn ConstructionScript)