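; BP_PNJ is an NPC character that offers a QTE to the player through a camera-facing widget.
; Look-at events show or hide the WB_QTE prompt and stop or restore walking, with a DoOnce guarding the spawn.
; InputA swaps in WB_EventA, forwards clicks after the first and locks BP_Princess movement until EndEvent.
; Movable NPCs it bumps are launched away, and Lover stores a follower index and disables sphere collision and radial pushes.
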(event OnComponentHit(CapsuleComponent)
  (params (HitComponent :type Primitive%20Component%20Object%20Reference) (OtherActor :type Actor%20Object%20Reference) (OtherComp :type Primitive%20Component%20Object%20Reference) (NormalImpulse :type Vector :default "0, 0, 0") (Hit :type Hit%20Result%20Structure%20%28by%20ref%29))
  (bind _asbp_pnj (Utilities|Casting|CastToBP_PNJ OtherActor))
  (if (== (Utilities|GetClass OtherActor) "BP_PNJ_C")
    (if (Variables|BP_PNJ_C|GetCanMove _asbp_pnj)
      (Character|LaunchCharacter _asbp_pnj (* (Math|Vector|Normalize (- (Transformation|GetActorLocation OtherActor) (Transformation|GetActorLocation))) 7.5e+02) false false))))

(event Custom|Reset
  (bind _widget (Variables|Default|GetWidget))
  (bind _returnvalue (UserInterface|GetWidget _widget))
  (bind _aswb_qte (Utilities|Casting|CastToWB_QTE _returnvalue))
  (Utilities|FlowControl|DoOnce false) ; enters at Reset
)

(event Custom|EndEvent
  (bind _widget (Variables|Default|GetWidget))
  (bind _returnvalue (UserInterface|CreateWidget "/Game/Global/UI/WB_QTE.WB_QTE_C"))
  (UserInterface|SetWidget _widget _returnvalue)
  (Development|SetHiddeninGame _widget true false)
  (Variables|Default|SetClick 0)
  (Variables|/Game/Global/Blueprint/Player/BP_Princess.BP_Princess_C|SetCanMoove (.AsBP%20Princess (Utilities|Casting|CastToBP_Princess (Game|Player|GetPlayerPawn 0))) true)
  (Variables|/Script/Engine.CharacterMovementComponent|SetMaxWalkSpeed (Variables|Character|GetCharacterMovement) 2.5e+02))

(event Custom|Lover
  (params (NumberIndex :type Integer))
  (bind _capsulecomponent (Variables|Collision|GetCapsuleComponent))
  (Variables|Default|SetIndexFollower NumberIndex)
  (Collision|SetCollisionEnabled (Variables|Default|GetSphere) "NoCollision")
  (Variables|/Script/Engine.PrimitiveComponent|SetbIgnoreRadialForce _capsulecomponent true)
  (Variables|/Script/Engine.PrimitiveComponent|SetbIgnoreRadialImpulse _capsulecomponent true))

(event EventBeginPlay)

(event Collision|EventActorBeginOverlap
  (params (OtherActor :type Actor%20Object%20Reference)))

(event EventTick
  (params (DeltaSeconds :type Float%20%28single-precision%29))
  (Transformation|SetWorldRotation (Variables|Default|GetWidget) (Math|Rotator|FindLookatRotation (Transformation|GetActorLocation) (Camera|GetCameraLocation (Game|GetPlayerCameraManager 0))) false false))

(event EventLookatPNJ
  (bind _widget (Variables|Default|GetWidget))
  (bind _returnvalue (UserInterface|GetWidget _widget))
  (bind _aswb_qte (Utilities|Casting|CastToWB_QTE _returnvalue))
  (Variables|Default|SetCanMove false)
  (Utilities|FlowControl|DoOnce false
    (:Completed
      (Development|SetHiddeninGame (Variables|Default|GetWidget) false false)
      (Utilities|IsValid _aswb_qte
        (:Is%20Valid
          (Default|SpawnAnim _aswb_qte)
          (Variables|Default|SetCanUnspawn true)
          (Variables|/Script/Engine.CharacterMovementComponent|SetMaxWalkSpeed (Variables|Character|GetCharacterMovement) 0.0))))))

(event EventStopLoockingPNJ
  (bind _widget (Variables|Default|GetWidget))
  (bind _returnvalue (UserInterface|GetWidget _widget))
  (bind _aswb_qte (Utilities|Casting|CastToWB_QTE _returnvalue))
  (Variables|Default|SetCanMove true)
  (Utilities|FlowControl|Delay 0.1)
  (if (Variables|Default|GetCanUnspawn)
    (Utilities|IsValid _aswb_qte
      (:Is%20Valid
        (Default|UnspawnAnim _aswb_qte)
        (Variables|Default|SetCanUnspawn false)
        (CallFunction|Reset)
        (Variables|/Script/Engine.CharacterMovementComponent|SetMaxWalkSpeed (Variables|Character|GetCharacterMovement) 2.5e+02)))))

(event EventInputA
  (bind _click (Variables|Default|GetClick))
  ;[1 1 1] Start qte slider
  (if (Variables|Default|GetCanUnspawn)
    (Default|UnspawnAnim (.AsWB%20QTE (Utilities|Casting|CastToWB_QTE (UserInterface|GetWidget (Variables|Default|GetWidget)))))
    (Variables|Default|SetCanUnspawn false)
    (CallFunction|Reset) ; reset animation spawn
    (bind _returnvalue (UserInterface|CreateWidget "/Game/Global/UI/WB_EventA.WB_EventA_C"))
    (UserInterface|SetWidget (Variables|Default|GetWidget) _returnvalue))
  (Utilities|IsValid _returnvalue
    (:Is%20Valid
      (Math|Integer|IncrementInt _click ; dodge first click
        (:%20%20
          (if (> _click 1)
            (Default|Click _returnvalue self) ; send to pnj the click button
          )
          (Variables|/Game/Global/Blueprint/Player/BP_Princess.BP_Princess_C|SetCanMoove (.AsBP%20Princess (Utilities|Casting|CastToBP_Princess (Game|Player|GetPlayerPawn 0))) false))))))

(fn ConstructionScript)