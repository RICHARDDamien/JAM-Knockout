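; BP_But is a goal zone where BP_Princess drops off her followers to score points.
; On box overlap, it adds the follower count to Points, then a DoOnce, reset on exit, gates the handoff.
; Each follower's blackboard is flagged and retargeted to the goal's location while the HUD and GI_Jam total update.
; The princess's follower list is then cleared and the player's lover count zeroed.
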(event OnComponentBeginOverlap(Box)
  (params (OverlappedComponent :type Primitive%20Component%20Object%20Reference) (OtherActor :type Actor%20Object%20Reference) (OtherComp :type Primitive%20Component%20Object%20Reference) (OtherBodyIndex :type Integer) (bFromSweep :type Boolean) (SweepResult :type Hit%20Result%20Structure%20%28by%20ref%29))
  (bind _asbp_princess (Utilities|Casting|CastToBP_Princess OtherActor))
  (bind _follower (Variables|/Game/Global/Blueprint/Player/BP_Princess.BP_Princess_C|GetFollower _asbp_princess))
  (if (== (Utilities|GetClass OtherActor) "/Game/Global/Blueprint/Player/BP_Princess.BP_Princess_C")
    (if (not (Utilities|Array|IsEmpty _follower))
      (Variables|Default|SetPoints (+ (Variables|Default|GetPoints) (Utilities|Array|Length _follower)))
      (Utilities|FlowControl|DoOnce false
        (:Completed
          (for _array_element _follower
            (AI|Components|Blackboard|SetValueasBool (AI|GetBlackboard _array_element) (Utilities|Name|MakeLiteralName "But") true)
            (AI|Components|Blackboard|SetValueasVector (AI|GetBlackboard _array_element) (Utilities|Name|MakeLiteralName "TargetToFollow") (Transformation|GetActorLocation))
            (bind _foundwidgets (Widget|GetAllWidgetsOfClass "/Game/Global/UI/Screen/WBP_HUD.WBP_HUD_C" true))
            (Default|PnjCountUpdate (Utilities|Array|Get(acopy) _foundwidgets))
            (Variables|/Game/Global/Blueprint/GI_Jam.GI_Jam_C|SetAmountOfLovers (.AsGI%20Jam (Utilities|Casting|CastToGI_Jam (Game|GetGameInstance))) (Variables|Default|GetPoints)))
          (Utilities|Array|Clear _follower)
          (Development|PrintString (Utilities|String|ToString(Integer) (Variables|Default|GetPoints)))
          (Variables|/Game/Global/Blueprint/Player/BP_Princess.BP_Princess_C|SetAmountOfLover (.AsBP%20Princess (Utilities|Casting|CastToBP_Princess (Game|Player|GetPlayerPawn 0))) 0))))))

(event OnComponentEndOverlap(Box)
  (params (OverlappedComponent :type Primitive%20Component%20Object%20Reference) (OtherActor :type Actor%20Object%20Reference) (OtherComp :type Primitive%20Component%20Object%20Reference) (OtherBodyIndex :type Integer))
  (if (== (Utilities|GetClass OtherActor) "/Game/Global/Blueprint/Player/BP_Princess.BP_Princess_C")
    (Utilities|FlowControl|DoOnce false) ; enters at Reset
  ))

(event EventBeginPlay)

(event Collision|EventActorBeginOverlap
  (params (OtherActor :type Actor%20Object%20Reference)))

(event EventTick
  (params (DeltaSeconds :type Float%20%28single-precision%29)))

(fn ConstructionScript)