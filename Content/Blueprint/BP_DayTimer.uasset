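; BP_DayTimer runs the endless maid-visit cycle: footsteps approach, the door opens on the maid, then closes and footsteps retreat.
; IsComming picks an approach time while a delayed loop raises footstep pitch through TimeCheck, and GoBack waits randomly before restarting it.
; Door and maid move on timelines, with open/close calls sent to BP_Princess.
; Higher Difficulty biases toward shorter approaches and more "fake" departures that reopen the door.
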(event Custom|OpenDoor
  (Audio|PlaySoundatLocation "/Game/SFX/DoorOpen.DoorOpen" (Transformation|GetWorldLocation (Variables|Default|GetDefaultSceneRoot)) "0, 0, 0" 1.0 1.0 0.0 0 0 0 0)
  (CallFunction|StopSound)
  (Variables|Default|SetSoundOn false)
  (Utilities|FlowControl|Delay 0.2)
  (Default|DoorOpen (.AsBP%20Princess (Utilities|Casting|CastToBP_Princess (Game|Player|GetPlayerPawn 0))))
  (Development|PrintString "OPEN_Door")
  (Utilities|FlowControl|Sequence
    (:then_0
      (bind _doortrack (Timeline|DoorOpening PlayFromStart)
        (:Update
          (Transformation|SetRelativeRotation (Variables|Default|GetDoor) (Math|Rotator|MakeRotator 0.0 0.0 (* _doortrack 9e+01)) false false))))
    (:then_1
      (bind _doortrack_2 (Timeline|MaidCome PlayFromStart)
        (:Update
          (Transformation|SetWorldLocation (Variables|Default|GetMaid) (Math|Vector|Lerp(Vector) (Variables|Default|GetLocation1) (Variables|Default|GetNew%20Location) _doortrack_2) false false))))))

(event Custom|CloseDoor
  (Audio|PlaySoundatLocation "/Game/SFX/DoorClose.DoorClose" (Transformation|GetWorldLocation (Variables|Default|GetDefaultSceneRoot)) "0, 0, 0" 1.0 1.0 0.0 0 0 0 0)
  (Default|DoorClose (.AsBP%20Princess (Utilities|Casting|CastToBP_Princess (Game|Player|GetPlayerPawn 0))))
  (Development|PrintString "CLOSE_Door")
  (Utilities|FlowControl|Sequence
    (:then_0
      (bind _doortrack (Timeline|DoorClosing ReverseFromEnd)
        (:Update
          (Transformation|SetRelativeRotation (Variables|Default|GetDoor) (Math|Rotator|MakeRotator 0.0 0.0 (* _doortrack 9e+01)) false false))))
    (:then_1
      (bind _doortrack_2 (Timeline|MaidGo ReverseFromEnd)
        (:Update
          (Transformation|SetWorldLocation (Variables|Default|GetMaid) (Math|Vector|Lerp(Vector) (Variables|Default|GetLocation1) (Variables|Default|GetNew%20Location) _doortrack_2) false false))))))

(event Custom|GoBack
  (CallFunction|PlaySoundGoBack)
  (Development|PrintString "GoBack")
  (Variables|Default|SetTimeGoBackLeft (Math|Random|RandomFloatinRange (Variables|Default|GetTimeBackMIN) (Variables|Default|GetTimeBackMAX)))
  (Utilities|FlowControl|Delay (Variables|Default|GetTimeGoBackLeft))
  (CallFunction|StopSound)
  (CallFunction|IsComming))

(event Custom|IsComming
  (bind _difficulty (Variables|Default|GetDifficulty))
  (bind _timecommingmin (Variables|Default|GetTimeCommingMIN))
  (bind _timecommingmax (Variables|Default|GetTimeCommingMAX))
  (bind _returnvalue (Math|Random|RandomFloatinRange _timecommingmin _timecommingmax))
  (bind _returnvalue_2 (/ _difficulty 2.0))
  (bind _returnvalue_3 (Math|Float|Lerp _returnvalue _timecommingmin _returnvalue_2))
  (Development|PrintString "Is Comming")
  (Variables|Default|SetSoundOn true)
  ;[1 1 1] Play sound foot comming
  (Variables|Default|SetTimeCommingLeft _returnvalue_3) ; random time left
  (Variables|Default|SetPitchMultiplier 0.001) ; reset start pitch
  (Variables|Default|SetDelayTime (Math|Float|MapRangeClamped _returnvalue_3 _timecommingmin _timecommingmax 0.01 0.1)) ; delay incursive func
  (CallFunction|PlaySoundFoot)
  (Utilities|FlowControl|Delay (Variables|Default|GetTimeCommingLeft))
  (CallFunction|OpenDoor)
  (Utilities|FlowControl|Delay (Variables|Default|GetOpeningDuration))
  (CallFunction|CloseDoor)
  ;[1 1 1] Fake or goback random
  (if (Math|Random|RandomBoolwithWeight (Math|Float|Lerp 0.9 0.3 (Variables|Default|GetDifficulty)))
    _
    (else
      (Development|PrintString "(FAKE)")
      (Utilities|FlowControl|Delay (Variables|Default|GetFakeTime))
      (CallFunction|OpenDoor)
      (Utilities|FlowControl|Delay (Variables|Default|GetOpeningDuration))
      (CallFunction|CloseDoor)))
  (CallFunction|GoBack))

(event Custom|PlaySoundFoot
  (bind _audioplayer (Variables|Default|GetAudioPlayer))
  (Audio|Components|Audio|SetSound _audioplayer "/Game/SFX/Cue_FootStep.Cue_FootStep")
  (Audio|Parameter|SetFloatParameter _audioplayer "ContinuousPitch" (Variables|Default|GetPitchMultiplier) :!class /Script/AudioExtensions.AudioParameterControllerInterface)
  (Audio|Components|Audio|FadeIn _audioplayer 0.1 1.0 0.0 "Linear" :!class /Script/Engine.AudioComponent)
  (bind _pitchcheck (CallFunction|TimeCheck :!label _label))
  (if (not _pitchcheck)
    (if (Variables|Default|GetSoundOn)
      (Utilities|FlowControl|Delay 0.2)
      (goto _label))))

(event Custom|StopSound
  (Audio|Components|Audio|Stop (Variables|Default|GetAudioPlayer)))

(event Custom|PlaySoundGoBack
  (bind _audioplayer (Variables|Default|GetAudioPlayer))
  (Audio|Components|Audio|SetSound _audioplayer "/Game/SFX/Cue_FootStep.Cue_FootStep")
  (Audio|Parameter|SetFloatParameter _audioplayer "ContinuousPitch" 0.2 :!class /Script/AudioExtensions.AudioParameterControllerInterface)
  (Audio|Components|Audio|FadeIn _audioplayer 0.1 1.0 0.0 "Linear" :!class /Script/Engine.AudioComponent))

(event EventBeginPlay
  ;[1 1 1] Begin play
  (CallFunction|IsComming))

(fn ConstructionScript)

(fn TimeCheck
  (bind _output_get (Variables|Default|SetPitchMultiplier (+ (Variables|Default|GetPitchMultiplier) 0.02)))
  (Audio|Parameter|SetFloatParameter (Variables|Default|GetAudioPlayer) "ContinuousPitch" _output_get :!class /Script/AudioExtensions.AudioParameterControllerInterface)
  (Development|PrintString (Utilities|String|ToString(Float) _output_get) true true "(R=0.000000,G=1.000000,B=0.091165,A=1.000000)")
  (return (>= _output_get 1.0)))